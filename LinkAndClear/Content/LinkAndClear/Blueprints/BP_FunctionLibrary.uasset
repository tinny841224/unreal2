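; Function library for a link-and-clear tile game that decides whether two grid cells can connect and be cleared.
; DoClear tries straight vertical or horizontal lines, then one-turn and two-turn paths, returning a type and turn-point IDs.
; Turn candidates come from scanning outward along passable "X:Y" map entries within GameInstance board bounds, with two-turn checks reusing the one-turn search.
; FillAllPathGrids expands path points into every intermediate cell ID.
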(fn IsSameGrid
  (params (_d1 :type ST%20Grid%20Data%20Structure) (_d2 :type ST%20Grid%20Data%20Structure))
  (bind (_value _grid_x _grid_y) (Utilities|Struct|BreakST_GridData _d1))
  (bind (_value_2 _grid_x_2 _grid_y_2) (Utilities|Struct|BreakST_GridData _d2))
  (Utilities|FlowControl|Sequence
    (:then_0
      (if (== _grid_x _grid_x_2)
        (if (== _grid_y _grid_y_2)
          (return true))))
    (:then_1
      (return false))))

(fn DoClear
  (params (_d1 :type ST%20Grid%20Data%20Structure) (_d2 :type ST%20Grid%20Data%20Structure) (_map :type Map%20of%20Strings%20to%20Objects))
  (Utilities|FlowControl|Sequence
    (:then_0
      (bind __clear (CallFunction|ClearbyVertical _d1 _d2 _map))
      (if __clear
        (return true "NewEnumerator0" 0)))
    (:then_1
      (bind __clear_2 (CallFunction|ClearbyHorizontal _d1 _d2 _map))
      (if __clear_2
        (return true "NewEnumerator1" 0)))
    (:then_2
      (bind (__clear_3 __type __ids) (CallFunction|ClearbyNodeI _d1 _d2 _map))
      (if __clear_3
        (return true "NewEnumerator2" __ids)))
    (:then_3
      (bind (__clear_4 __type_2 __ids_2) (CallFunction|ClearbyNodeII _d1 _d2 _map))
      (if __clear_4
        (return true "NewEnumerator3" __ids_2)))
    (:then_4
      (return false "NewEnumerator4" 0))))

(fn ClearbyVertical
  (params (_d1 :type ST%20Grid%20Data%20Structure) (_d2 :type ST%20Grid%20Data%20Structure) (_map :type Map%20of%20Strings%20to%20Objects))
  (bind (_value _grid_x _grid_y) (Utilities|Struct|BreakST_GridData _d1))
  (bind (_value_2 _grid_x_2 _grid_y_2) (Utilities|Struct|BreakST_GridData _d2))
  (bind _returnvalue (Math|Integer|Min(Integer) _grid_y _grid_y_2))
  (bind _returnvalue_2 (Math|Integer|Max(Integer) _grid_y _grid_y_2))
  (bind _returnvalue_3 (CallFunction|ClearbyVerticalNearby _d1 _d2))
  (if _returnvalue_3
    (return true)
    (else
      (Utilities|FlowControl|Sequence
        (:then_0
          (if (== _grid_x _grid_x_2)
            (bind _output_get (LocalVariables|Settmp_x _grid_x))
            (if (<= (- _returnvalue_2 _returnvalue) 1)
              (return true)
              (else
                (for _index (range (+ _returnvalue 1) (- _returnvalue_2 1))
                  (if (not (.ReturnValue (Utilities|Map|Find _map (Utilities|String|Append (Utilities|String|ToString(Integer) _output_get) ":" (Utilities|String|ToString(Integer) _index)))))
                    (return false)))
                (return true)))))
        (:then_1
          (return false))))))

(fn ClearbyVerticalNearby
  (params (_d1 :type ST%20Grid%20Data%20Structure) (_d2 :type ST%20Grid%20Data%20Structure))
  (bind (_value _grid_x _grid_y) (Utilities|Struct|BreakST_GridData _d1))
  (bind (_value_2 _grid_x_2 _grid_y_2) (Utilities|Struct|BreakST_GridData _d2))
  (Utilities|FlowControl|Sequence
    (:then_0
      (if (== _grid_x _grid_x_2)
        (if (<= (Math|Integer|Absolute(Integer) (- _grid_y _grid_y_2)) 1)
          (return true))))
    (:then_1
      (return false))))

(fn ClearbyHorizontal
  (params (_d1 :type ST%20Grid%20Data%20Structure) (_d3 :type ST%20Grid%20Data%20Structure) (_map :type Map%20of%20Strings%20to%20Objects))
  (bind (_value _grid_x _grid_y) (Utilities|Struct|BreakST_GridData _d1))
  (bind (_value_2 _grid_x_2 _grid_y_2) (Utilities|Struct|BreakST_GridData _d3))
  (bind _returnvalue (Math|Integer|Min(Integer) _grid_x _grid_x_2))
  (bind _returnvalue_2 (Math|Integer|Max(Integer) _grid_x _grid_x_2))
  (bind _returnvalue_3 (CallFunction|ClearbyHorizontalNearby _d1 _d3))
  (if _returnvalue_3
    (return true)
    (else
      (Utilities|FlowControl|Sequence
        (:then_0
          (if (== _grid_y _grid_y_2)
            (bind _output_get (LocalVariables|Settmp_y _grid_y))
            (if (<= (- _returnvalue_2 _returnvalue) 1)
              (return true)
              (else
                (for _index (range (+ _returnvalue 1) (- _returnvalue_2 1))
                  (if (not (.ReturnValue (Utilities|Map|Find _map (Utilities|String|Append (Utilities|String|ToString(Integer) _index) ":" (Utilities|String|ToString(Integer) _output_get)))))
                    (return false)))
                (return true)))))
        (:then_1
          (return false))))))

(fn ClearbyHorizontalNearby
  (params (_d1 :type ST%20Grid%20Data%20Structure) (_d2 :type ST%20Grid%20Data%20Structure))
  (bind (_value _grid_x _grid_y) (Utilities|Struct|BreakST_GridData _d1))
  (bind (_value_2 _grid_x_2 _grid_y_2) (Utilities|Struct|BreakST_GridData _d2))
  (Utilities|FlowControl|Sequence
    (:then_0
      (if (== _grid_y _grid_y_2)
        (if (<= (Math|Integer|Absolute(Integer) (- _grid_x _grid_x_2)) 1)
          (return true))))
    (:then_1
      (return false))))

(fn ClearbyNodeI
  (params (_d1 :type ST%20Grid%20Data%20Structure) (_d2 :type ST%20Grid%20Data%20Structure) (_map :type Map%20of%20Strings%20to%20Objects))
  (Utilities|FlowControl|Sequence
    (:then_0
      (bind (__clear __ids) (CallFunction|ClearbyVerticalInsert _d1 _d2 _map))
      (if __clear
        (return true "NewEnumerator5" __ids)))
    (:then_1
      (bind (__clear_2 __ids_2) (CallFunction|ClearbyHorizontalInsert _d1 _d2 _map))
      (if __clear_2
        (return true "NewEnumerator6" __ids_2)))
    (:then_2
      (return false "NewEnumerator4" 0))))

(fn ClearbyVerticalInsert
  (params (_d11 :type ST%20Grid%20Data%20Structure) (_d22 :type ST%20Grid%20Data%20Structure) (_map22 :type Map%20of%20Strings%20to%20Objects))
  (bind _tmp_ids (LocalVariables|Gettmp_ids))
  (bind _output_get (LocalVariables|Sets_grid _d11))
  (bind _output_get_2 (LocalVariables|Sete_grid _d22))
  (bind __grids (CallFunction|GetVerticalInsertGrids _output_get _output_get_2 _map22))
  (for _array_element __grids
    (bind _output_get_3 (LocalVariables|Settmp_grid _array_element))
    (bind __clear (CallFunction|ClearbyVertical (LocalVariables|Gets_grid) _output_get_3 _map22))
    (if __clear
      (bind __clear_2 (CallFunction|ClearbyHorizontal (LocalVariables|Gete_grid) _output_get_3 _map22))
      (if __clear_2
        (bind __id (CallFunction|GetPositionID (.Grid_X (Utilities|Struct|BreakST_GridData _output_get_3)) (.Grid_Y (Utilities|Struct|BreakST_GridData _output_get_3))))
        (Utilities|Array|Add _tmp_ids __id)
        (return true _tmp_ids))))
  (return false 0))

(fn GetVerticalInsertGrids
  (params (_d1 :type ST%20Grid%20Data%20Structure) (_d2 :type ST%20Grid%20Data%20Structure) (_map :type Map%20of%20Strings%20to%20Objects))
  (bind (_value _grid_x _grid_y) (Utilities|Struct|BreakST_GridData _d1))
  (bind _res_grids (LocalVariables|Getres_grids))
  (LocalVariables|Settmp_x _grid_x)
  (Utilities|FlowControl|Sequence
    (:then_0
      (bind _output_get (LocalVariables|Settmp_y _grid_y))
      (Math|Integer|DecrementInt _output_get
        (:%20%20
          (while (>= (LocalVariables|Gettmp_y) 0)
            (bind __id (CallFunction|GetPositionID (LocalVariables|Gettmp_x) (LocalVariables|Gettmp_y)))
            (if (.ReturnValue (Utilities|Map|Find _map __id))
              (Utilities|Array|Add _res_grids (Utilities|Struct|MakeST_GridData -1 (LocalVariables|Gettmp_x) (LocalVariables|Gettmp_y)))
              (Math|Integer|DecrementInt (LocalVariables|Gettmp_y))
              (else
                (LocalVariables|Settmp_y -1)))))))
    (:then_1
      (bind _output_get_2 (LocalVariables|Settmp_y _grid_y))
      (Math|Integer|IncrementInt _output_get_2
        (:%20%20
          (bind _asbp_game_instance (Utilities|Casting|CastToBP_GameInstance (Game|GetGameInstance)))
          (while (> (Variables|/Game/LinkAndClear/Blueprints/BP_GameInstance.BP_GameInstance_C|GetVerticalSize _asbp_game_instance) (LocalVariables|Gettmp_y))
            (bind __id_2 (CallFunction|GetPositionID (LocalVariables|Gettmp_x) (LocalVariables|Gettmp_y)))
            (if (.ReturnValue (Utilities|Map|Find _map __id_2))
              (Utilities|Array|Add _res_grids (Utilities|Struct|MakeST_GridData -1 (LocalVariables|Gettmp_x) (LocalVariables|Gettmp_y)))
              (Math|Integer|IncrementInt (LocalVariables|Gettmp_y))
              (else
                (LocalVariables|Settmp_y (Variables|/Game/LinkAndClear/Blueprints/BP_GameInstance.BP_GameInstance_C|GetVerticalSize _asbp_game_instance))))))))
    (:then_2
      (return (LocalVariables|Getres_grids)))))

(fn GetPositionID
  (params (_x :type Integer) (_y :type Integer))
  (return (Utilities|String|Append (Utilities|String|ToString(Integer) _x) ":" (Utilities|String|ToString(Integer) _y))))

(fn ClearbyHorizontalInsert
  (params (_d11 :type ST%20Grid%20Data%20Structure) (_d22 :type ST%20Grid%20Data%20Structure) (_map22 :type Map%20of%20Strings%20to%20Objects))
  (bind _tmp_ids (LocalVariables|Gettmp_ids))
  (bind _output_get (LocalVariables|Sets_grid _d11))
  (bind _output_get_2 (LocalVariables|Sete_grid _d22))
  (bind __grids (CallFunction|GetHorizontalInsertGrids _output_get _output_get_2 _map22))
  (for _array_element __grids
    (bind _output_get_3 (LocalVariables|Settmp_grid _array_element))
    (bind __clear (CallFunction|ClearbyHorizontal (LocalVariables|Gets_grid) _output_get_3 _map22))
    (if __clear
      (bind __clear_2 (CallFunction|ClearbyVertical (LocalVariables|Gete_grid) _output_get_3 _map22))
      (if __clear_2
        (bind __id (CallFunction|GetPositionID (.Grid_X (Utilities|Struct|BreakST_GridData _output_get_3)) (.Grid_Y (Utilities|Struct|BreakST_GridData _output_get_3))))
        (Utilities|Array|Add _tmp_ids __id)
        (return true _tmp_ids))))
  (return false 0))

(fn GetHorizontalInsertGrids
  (params (_d11 :type ST%20Grid%20Data%20Structure) (_d22 :type ST%20Grid%20Data%20Structure) (_map22 :type Map%20of%20Strings%20to%20Objects))
  (bind (_value _grid_x _grid_y) (Utilities|Struct|BreakST_GridData _d11))
  (bind _res_grids (LocalVariables|Getres_grids))
  (LocalVariables|Settmp_y _grid_y)
  (Utilities|FlowControl|Sequence
    (:then_0
      (bind _output_get (LocalVariables|Settmp_x _grid_x))
      (Math|Integer|DecrementInt _output_get
        (:%20%20
          (while (>= (LocalVariables|Gettmp_x) 0)
            (bind __id (CallFunction|GetPositionID (LocalVariables|Gettmp_x) (LocalVariables|Gettmp_y)))
            (if (.ReturnValue (Utilities|Map|Find _map22 __id))
              (Utilities|Array|Add _res_grids (Utilities|Struct|MakeST_GridData -1 (LocalVariables|Gettmp_x) (LocalVariables|Gettmp_y)))
              (Math|Integer|DecrementInt (LocalVariables|Gettmp_x))
              (else
                (LocalVariables|Settmp_x -1)))))))
    (:then_1
      (bind _output_get_2 (LocalVariables|Settmp_x _grid_x))
      (Math|Integer|IncrementInt _output_get_2
        (:%20%20
          (bind _asbp_game_instance (Utilities|Casting|CastToBP_GameInstance (Game|GetGameInstance)))
          (while (> (Variables|/Game/LinkAndClear/Blueprints/BP_GameInstance.BP_GameInstance_C|GetHorizontalSize _asbp_game_instance) (LocalVariables|Gettmp_x))
            (bind __id_2 (CallFunction|GetPositionID (LocalVariables|Gettmp_x) (LocalVariables|Gettmp_y)))
            (if (.ReturnValue (Utilities|Map|Find _map22 __id_2))
              (Utilities|Array|Add _res_grids (Utilities|Struct|MakeST_GridData -1 (LocalVariables|Gettmp_x) (LocalVariables|Gettmp_y)))
              (Math|Integer|IncrementInt (LocalVariables|Gettmp_x))
              (else
                (LocalVariables|Settmp_x (Variables|/Game/LinkAndClear/Blueprints/BP_GameInstance.BP_GameInstance_C|GetHorizontalSize _asbp_game_instance))))))))
    (:then_2
      (return (LocalVariables|Getres_grids)))))

(fn ClearbyNodeII
  (params (_d1 :type ST%20Grid%20Data%20Structure) (_d2 :type ST%20Grid%20Data%20Structure) (_map :type Map%20of%20Strings%20to%20Objects))
  (bind __grids (CallFunction|GetInsertGrids _d1 _map))
  (for _array_element __grids
    (bind (__clear __type __ids) (CallFunction|ClearbyNodeI _array_element _d2 _map))
    (if __clear
      (bind _output_get (LocalVariables|Setres_grids __ids))
      (bind __id (CallFunction|GetPositionID (.Grid_X (Utilities|Struct|BreakST_GridData _array_element)) (.Grid_Y (Utilities|Struct|BreakST_GridData _array_element))))
      (Utilities|Array|Insert _output_get __id)
      (return true "NewEnumerator3" _output_get)))
  (return false "NewEnumerator4" 0))

(fn GetInsertGrids
  (params (_d1 :type ST%20Grid%20Data%20Structure) (_map :type Map%20of%20Strings%20to%20Objects))
  (bind _res_grids (LocalVariables|Getres_grids))
  (bind __grids (CallFunction|GetHorizontalInsertGrids :_d11 _d1 :_map22 _map))
  (Utilities|Array|AppendArray _res_grids __grids)
  (bind __grids_2 (CallFunction|GetVerticalInsertGrids :_d1 _d1 :_map _map))
  (Utilities|Array|AppendArray _res_grids __grids_2)
  (return _res_grids))

(fn FillAllPathGrids
  (params (_ids :type Array%20of%20Strings))
  (bind _res_ids (LocalVariables|Getres_ids))
  (bind _res_ids_2 (LocalVariables|Getres_ids))
  (bind _output_get (LocalVariables|Settmp_ids _ids))
  (Utilities|Array|Clear (LocalVariables|Getres_ids))
  (for _index (range 0 (- (Utilities|Array|Length _output_get) 2))
    (Utilities|Array|Add _res_ids_2 (Utilities|Array|Get(acopy) (LocalVariables|Gettmp_ids) _index))
    (bind _res_ids2 (CallFunction|FillPathGridsBetween (Utilities|Array|Get(acopy) (LocalVariables|Gettmp_ids) _index) (Utilities|Array|Get(acopy) (LocalVariables|Gettmp_ids) (+ _index 1))))
    (Utilities|Array|AppendArray _res_ids_2 _res_ids2))
  (Utilities|Array|Add _res_ids (Utilities|Array|Get(acopy) _output_get (- (Utilities|Array|Length _output_get) 1)))
  (return _res_ids))

(fn FillPathGridsBetween
  (params (id1 :type String) (id2 :type String))
  (bind _returnvalue (Utilities|String|ParseIntoArray id2 ":"))
  (bind _returnvalue_2 (Utilities|String|ParseIntoArray id1 ":"))
  (bind _output (Utilities|Array|Get(acopy) _returnvalue_2))
  (bind _output_2 (Utilities|Array|Get(acopy) _returnvalue))
  (bind _output_3 (Utilities|Array|Get(acopy) _returnvalue_2 1))
  (bind _output_4 (Utilities|Array|Get(acopy) _returnvalue 1))
  (bind _returnvalue_3 (Math|Conversions|ToInteger(Byte) _output_4))
  (bind _returnvalue_4 (Math|Conversions|ToInteger(Byte) _output))
  (bind _returnvalue_5 (Math|Conversions|ToInteger(Byte) _output_2))
  (bind _returnvalue_6 (Math|Conversions|ToInteger(Byte) _output_3))
  (if (== _returnvalue_4 _returnvalue_5)
    (bind _res_ids (CallFunction|FillVerticalPathGrids _returnvalue_4 _returnvalue_6 _returnvalue_5 _returnvalue_3))
    (return _res_ids)
    (elif (== _returnvalue_6 _returnvalue_3)
      (bind _res_ids_2 (CallFunction|FillHorizontalPathGrids _returnvalue_4 _returnvalue_6 _returnvalue_5 _returnvalue_3))
      (return _res_ids_2)
      (else
        (return 0)))))

(fn FillVerticalPathGrids
  (params (_s_x :type Integer) (_s_y :type Integer) (_e_x :type Integer) (_e_y :type Integer))
  (bind _returnvalue (> _s_y _e_y))
  (LocalVariables|Settmp_x _s_x)
  (bind _output_get (LocalVariables|Settmp_y _s_y))
  (if _returnvalue
    (Math|Integer|DecrementInt _output_get
      (:%20%20
        _))
    (else
      (Math|Integer|IncrementInt _output_get
        (:%20%20
          _))))
  (while (!= _output_get _e_y)
    (bind __id (CallFunction|GetPositionID (LocalVariables|Gettmp_x) (LocalVariables|Gettmp_y)))
    (Utilities|Array|Add (LocalVariables|Gettmp_ids) __id)
    (if _returnvalue
      (Math|Integer|DecrementInt (LocalVariables|Gettmp_y))
      (else
        (Math|Integer|IncrementInt (LocalVariables|Gettmp_y)))))
  (return (LocalVariables|Gettmp_ids)))

(fn FillHorizontalPathGrids
  (params (_s_x :type Integer) (_s_y :type Integer) (_e_x :type Integer) (_e_y :type Integer))
  (bind _returnvalue (> _s_x _e_x))
  (LocalVariables|Settmp_y _s_y)
  (bind _output_get (LocalVariables|Settmp_x _s_x))
  (if _returnvalue
    (Math|Integer|DecrementInt _output_get
      (:%20%20
        _))
    (else
      (Math|Integer|IncrementInt _output_get
        (:%20%20
          _))))
  (while (!= _output_get _e_x)
    (bind __id (CallFunction|GetPositionID (LocalVariables|Gettmp_x) (LocalVariables|Gettmp_y)))
    (Utilities|Array|Add (LocalVariables|Gettmp_ids) __id)
    (if _returnvalue
      (Math|Integer|DecrementInt (LocalVariables|Gettmp_x))
      (else
        (Math|Integer|IncrementInt (LocalVariables|Gettmp_x)))))
  (return (LocalVariables|Gettmp_ids)))