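; BPGameMode is a game mode that sets up mouse input and the UI when play begins.
; It enables the cursor and click events, then creates the BPEase and BPMain widgets, showing the first and hiding the second.
; Both widget references are stored on BPGameInstance.
; Every tick it calls TweentoOnTick to drive Tweento updates.
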(event EventBeginPlay
  (bind _returnvalue (Game|GetPlayerController 0))
  (Variables|/Script/Engine.PlayerController|SetbEnableClickEvents _returnvalue true)
  (Variables|/Script/Engine.PlayerController|SetbShowMouseCursor _returnvalue true)
  (bind _asbpgame_instance (Utilities|Casting|CastToBPGameInstance (Game|GetGameInstance)))
  (Utilities|FlowControl|Sequence
    (:then_0
      (bind _returnvalue_2 (UserInterface|CreateWidget "/Game/Game/Blueprints/BPEase.BPEase_C"))
      (UserInterface|Viewport|AddtoViewport _returnvalue_2 0)
      (Widget|SetVisibility _returnvalue_2 "Visible")
      (Variables|/Game/Game/Blueprints/BPGameInstance.BPGameInstance_C|SetBPEASE _asbpgame_instance _returnvalue_2))
    (:then_1
      (bind _returnvalue_3 (UserInterface|CreateWidget "/Game/Game/Blueprints/BPMain.BPMain_C"))
      (UserInterface|Viewport|AddtoViewport _returnvalue_3 0)
      (Widget|SetVisibility _returnvalue_3 "Hidden")
      (Variables|/Game/Game/Blueprints/BPGameInstance.BPGameInstance_C|SetBPMAIN _asbpgame_instance _returnvalue_3))))

(event EventTick
  (params (DeltaSeconds :type Float%20%28single-precision%29))
  (CallFunction|TweentoonTick))

(fn ConstructionScript)