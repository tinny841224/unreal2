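; BP_PlayerControl forwards player movement input to the game mode in the RPG2D Carmack map sample.
; It listens to the MoveUp and MoveRight axes and ignores zero values.
; Non-zero values go to OnMoveUp and OnMoveRight on BP_GameMode through a cast of the current game mode, so this Blueprint moves nothing itself.
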(event EventBeginPlay)

(event EventTick
  (params (DeltaSeconds :type Float%20%28single-precision%29)))

(event Input|AxisEvents|InputAxisMoveUp
  (params (AxisValue :type Float%20%28single-precision%29))
  (if (!= AxisValue 0.0)
    (bind _asbp_game_mode (Utilities|Casting|CastToBP_GameMode (Game|GetGameMode)))
    (Default|OnMoveUp _asbp_game_mode AxisValue)))

(event Input|AxisEvents|InputAxisMoveRight
  (params (AxisValue :type Float%20%28single-precision%29))
  (if (!= AxisValue 0.0)
    (bind _asbp_game_mode (Utilities|Casting|CastToBP_GameMode (Game|GetGameMode)))
    (Default|OnMoveRight _asbp_game_mode AxisValue)))

(fn ConstructionScript)