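; BP_GameMode is the game mode for the RPG2DCarmackMap game, setting up the main UI and relaying movement to it.
; On BeginPlay it shows the mouse cursor, enables click events, then creates the BP_Main widget, adds it to the viewport and keeps a reference.
; Its OnMoveUp and OnMoveRight functions forward axis values straight to that widget, so movement handling lives in BP_Main rather than here.
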(event EventBeginPlay
  (bind _returnvalue (Game|GetPlayerController 0))
  (Variables|/Script/Engine.PlayerController|SetbShowMouseCursor _returnvalue true)
  (Variables|/Script/Engine.PlayerController|SetbEnableClickEvents _returnvalue true)
  (bind _returnvalue_2 (UserInterface|CreateWidget "/Game/RPG2DCarmackMap/Blueprints/BP_Main.BP_Main_C"))
  (UserInterface|Viewport|AddtoViewport _returnvalue_2 0)
  (Variables|Default|SetBPMAIN _returnvalue_2))

(event EventTick
  (params (DeltaSeconds :type Float%20%28single-precision%29)))

(fn ConstructionScript)

(fn OnMoveUp
  (params (_val :type Float%20%28single-precision%29))
  (Default|OnMoveUp (Variables|Default|GetBPMAIN) _val))

(fn OnMoveRight
  (params (_val :type Float%20%28single-precision%29))
  (Default|OnMoveRight (Variables|Default|GetBPMAIN) _val))