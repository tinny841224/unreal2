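; Tweento function library that tweens UMG widgets' canvas position, render transform and opacity between A/B values using a selectable ease.
; AddWidgetToTweentoList stores timed actions on BPGameInstance and applies their starting state.
; TweentoTick is meant to advance actions by elapsed time, snap finished ones to the end and remove them, but its logic after the cast is disconnected.
; The end-callback cast is an unset, project-specific placeholder.
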(fn PlayTweentoVec
  (params (_para :type Tweento%20Para%20Struct%20Structure) (_f :type Float%20%28single-precision%29) (_widget :type Widget%20Object%20Reference) (_ease :type EEasingFunc%20Enum :default "Linear"))
  (bind (_tweentoid _b_value _value_a _value_b _b_vec _vec_a _vec_b) (Utilities|Struct|BreakTweentoParaStruct _para))
  (bind _result (Math|Interpolation|Ease _ease _f _vec_a _vec_b 2.0))
  (bind (_x _y) (Math|Vector|BreakVector _result))
  (if _b_vec
    (Class|CanvasPanelSlot|SetPosition (Class|WidgetLayoutLibrary|SlotasCanvasSlot _widget) (Math|Vector2D|MakeVector2D _x _y))))

(fn PlayTweentoTransform
  (params (_para :type Tweento%20Para%20Struct%20Structure) (_f :type Float%20%28single-precision%29) (_widget :type Widget%20Object%20Reference) (_ease :type EEasingFunc%20Enum :default "Linear"))
  (bind (_tweentoid _b_value _value_a _value_b _b_vec _vec_a _vec_b _uwtransform _uwtranslation_a _uwtranslation_b _uwscale_a _uwscale_b _uwangle_a _uwangle_b) (Utilities|Struct|BreakTweentoParaStruct _para))
  (if _uwtransform
    (bind __vec2d (CallFunction|GetEaseVec2DfromVec _ease _f _uwtranslation_a _uwtranslation_b))
    (bind __vec2d_2 (CallFunction|GetEaseVec2DfromVec _ease _f _uwscale_a _uwscale_b))
    (bind __angle (CallFunction|GetEaseAngle _ease _f _uwangle_a _uwangle_b))
    (Class|Widget|SetRenderTransform _widget (Utilities|Struct|MakeWidgetTransform __vec2d __vec2d_2 "(X=0.000000,Y=0.000000)" __angle))))

(fn GetEaseVec2DfromVec
  (params (_ease :type EEasingFunc%20Enum :default "Linear") (_f :type Float%20%28single-precision%29) (_vec_a :type Vector) (_vec_b :type Vector))
  (bind _result (Math|Interpolation|Ease _ease _f _vec_a _vec_b 2.0))
  (bind (_x _y) (Math|Vector|BreakVector _result))
  (return (Math|Vector2D|MakeVector2D _x _y)))

(fn GetEaseAngle
  (params (_ease :type EEasingFunc%20Enum :default "Linear") (_f :type Float%20%28single-precision%29) (_angle_a :type Float%20%28single-precision%29) (_abgle_b :type Float%20%28single-precision%29))
  (return (Math|Interpolation|Ease _ease _f _angle_a _abgle_b 2.0)))

(fn PlayOpacity
  (params (_para :type Tweento%20Para%20Struct%20Structure) (_f :type Float%20%28single-precision%29) (_widget :type Widget%20Object%20Reference) (_ease :type EEasingFunc%20Enum :default "Linear"))
  (bind (_tweentoid _b_value _value_a _value_b _b_vec _vec_a _vec_b _uwtransform _uwtranslation_a _uwtranslation_b _uwscale_a _uwscale_b _uwangle_a _uwangle_b _b_beziar _beziarvec2s _b_opacity _opacity_a _opacity_b) (Utilities|Struct|BreakTweentoParaStruct _para))
  (if _b_opacity
    (Widget|SetRenderOpacity _widget (Math|Interpolation|Ease _ease _f _opacity_a _opacity_b 2.0))))

(fn GetF
  (params (_s :type Float%20%28single-precision%29) (_e :type Float%20%28single-precision%29))
  (return (/ (- (Utilities|Time|GetTimeSeconds) _s) (- _e _s))))

(fn PlayTweento
  (params (_para :type Tweento%20Para%20Struct%20Structure) (_f :type Float%20%28single-precision%29) (_widget :type Widget%20Object%20Reference) (_ease :type EEasingFunc%20Enum :default "Linear"))
  (Utilities|FlowControl|Sequence
    (:then_0
      (Para|PlayTweentoVec _para _f _widget _ease))
    (:then_1
      (Para|PlayTweentoTransform _para _f _widget _ease))
    (:then_2
      (Para|PlayOpacity _para _f _widget _ease))))

(fn TweentoTick
  (bind _asbpgame_instance (Utilities|Casting|CastToBPGameInstance (Game|GetGameInstance))))

(fn AddWidgettoTweentoList
  (params (_delay :type Float%20%28single-precision%29) (_widget :type Widget%20Object%20Reference) (_para :type Array%20of%20Tweento%20Para%20Struct%20Structures) (_ease :type EEasingFunc%20Enum :default "Linear") (_cnt_id :type Name))
  (bind _returnvalue (Utilities|Time|GetTimeSeconds))
  (bind _asbpgame_instance (Utilities|Casting|CastToBPGameInstance (Game|GetGameInstance)))
  (Utilities|Array|Add (Variables|/Game/Blueprints/BPGameInstance.BPGameInstance_C|GetTweentoActionList _asbpgame_instance) (Utilities|Struct|MakeTweentoActionStruct _widget _returnvalue (+ _delay _returnvalue) _para _ease true "NewEnumerator0" "None" _cnt_id))
  (for _array_element _para
    (CallFunction|PlayTweento _array_element 0.0 _widget _ease)))