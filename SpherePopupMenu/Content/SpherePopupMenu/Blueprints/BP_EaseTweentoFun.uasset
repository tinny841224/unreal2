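; Tween function library that animates UMG widget transform, canvas position, opacity, angle and image color with selectable easing curves.
; PlayWidget functions queue timed actions in BP_EaseInstance's TweentoActionList on the game instance.
; TweentoOnTick computes eased progress and applies each property, then snaps expired actions to their end, notifies the BP_MenuItem and removes them.
; Bezier paths of any point count use Bernstein polynomials to set canvas position.
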(fn PlayTweentoTransform
  (params (_para :type ST%20Ease%20Tweento%20Para%20Struct%20Structure) (_c_f :type Float%20%28single-precision%29) (_widget :type Widget%20Object%20Reference))
  (bind (_type_value _valuea _valueb _type_vector2d _vector2da _vector2db _type_transform _translationa _translationb _scalea _scaleb _sheara _shearb _type_angle _anglea _angleb) (Utilities|Struct|BreakST_EaseTweentoParaStruct _para))
  (if _type_transform
    (bind __res (Global|GetCustomEaseVec2D _c_f _translationa _translationb))
    (bind __res_2 (Global|GetCustomEaseVec2D _c_f _scalea _scaleb))
    (bind __res_3 (Global|GetCustomEaseVec2D _c_f _sheara _shearb))
    (bind __res_4 (Global|GetCustomEaseFloat _c_f _anglea _angleb))
    (Class|Widget|SetRenderTransform _widget (Utilities|Struct|MakeWidgetTransform __res __res_2 __res_3 __res_4))))

(fn PlayTweentoVec
  (params (_para :type ST%20Ease%20Tweento%20Para%20Struct%20Structure) (_c_f :type Float%20%28single-precision%29) (_widget :type Widget%20Object%20Reference))
  (bind (_type_value _valuea _valueb _type_vector2d _vector2da _vector2db) (Utilities|Struct|BreakST_EaseTweentoParaStruct _para))
  (bind _returnvalue (Class|WidgetLayoutLibrary|SlotasCanvasSlot _widget))
  (if _type_vector2d
    (bind __res (Global|GetCustomEaseVec2D _c_f _vector2da _vector2db))
    (if (Utilities|IsValid _returnvalue)
      (Class|CanvasPanelSlot|SetPosition _returnvalue __res))))

(fn PlayOpacity
  (params (_para :type ST%20Ease%20Tweento%20Para%20Struct%20Structure) (_c_f :type Float%20%28single-precision%29) (_widget :type Widget%20Object%20Reference))
  (bind (_type_value _valuea _valueb _type_vector2d _vector2da _vector2db _type_transform _translationa _translationb _scalea _scaleb _sheara _shearb _type_angle _anglea _angleb _type_opacity _opacitya _opacityb) (Utilities|Struct|BreakST_EaseTweentoParaStruct _para))
  (if _type_opacity
    (bind __res (Global|GetCustomEaseFloat _c_f _opacitya _opacityb))
    (Widget|SetRenderOpacity _widget __res)))

(fn PlayTweento
  (params (_para :type ST%20Ease%20Tweento%20Para%20Struct%20Structure) (_c_f :type Float%20%28single-precision%29) (_widget :type Widget%20Object%20Reference))
  (Utilities|FlowControl|Sequence
    (:then_0
      (Para|PlayTweentoTransform _para _c_f _widget))
    (:then_1
      (Para|PlayTweentoVec _para _c_f _widget))
    (:then_2
      (Para|PlayOpacity _para _c_f _widget))
    (:then_3
      (Para|PlayAngle _para _c_f _widget))
    (:then_5
      (Para|PlayColorandOpacity _para _c_f _widget))
    (:then_6
      (Para|PlayBeziar _para _c_f _widget))))

(fn TweentoonTick
  (bind _asbp_ease_instance (Utilities|Casting|CastToBP_EaseInstance (Game|GetGameInstance)))
  (if (> (Utilities|Array|Length (Variables|/Game/SpherePopupMenu/Blueprints/BP_EaseInstance.BP_EaseInstance_C|GetTweentoActionList _asbp_ease_instance)) 0)
    (for _index (range 0 (- (Utilities|Array|Length (Variables|/Game/SpherePopupMenu/Blueprints/BP_EaseInstance.BP_EaseInstance_C|GetTweentoActionList _asbp_ease_instance)) 1))
      (bind __c_f (Global|GetCustomF (.S_Time (Utilities|Struct|BreakST_EaseTweentoActionStruct (Utilities|Array|Get(acopy) (Variables|/Game/SpherePopupMenu/Blueprints/BP_EaseInstance.BP_EaseInstance_C|GetTweentoActionList _asbp_ease_instance) _index))) (.E_Time (Utilities|Struct|BreakST_EaseTweentoActionStruct (Utilities|Array|Get(acopy) (Variables|/Game/SpherePopupMenu/Blueprints/BP_EaseInstance.BP_EaseInstance_C|GetTweentoActionList _asbp_ease_instance) _index))) (.CEase (Utilities|Struct|BreakST_EaseTweentoActionStruct (Utilities|Array|Get(acopy) (Variables|/Game/SpherePopupMenu/Blueprints/BP_EaseInstance.BP_EaseInstance_C|GetTweentoActionList _asbp_ease_instance) _index)))))
      (for _array_element (.ParaList (Utilities|Struct|BreakST_EaseTweentoActionStruct (Utilities|Array|Get(acopy) (Variables|/Game/SpherePopupMenu/Blueprints/BP_EaseInstance.BP_EaseInstance_C|GetTweentoActionList _asbp_ease_instance) _index)))
        (Global|PlayTweento _array_element __c_f (.Widget (Utilities|Struct|BreakST_EaseTweentoActionStruct (Utilities|Array|Get(acopy) (Variables|/Game/SpherePopupMenu/Blueprints/BP_EaseInstance.BP_EaseInstance_C|GetTweentoActionList _asbp_ease_instance) _index))))))
    (for _index_2 (range 0 (- (Utilities|Array|Length (Variables|/Game/SpherePopupMenu/Blueprints/BP_EaseInstance.BP_EaseInstance_C|GetTweentoActionList _asbp_ease_instance)) 1))
      (if (> (Utilities|Time|GetTimeSeconds) (.E_Time (Utilities|Struct|BreakST_EaseTweentoActionStruct (Utilities|Array|Get(acopy) (Variables|/Game/SpherePopupMenu/Blueprints/BP_EaseInstance.BP_EaseInstance_C|GetTweentoActionList _asbp_ease_instance) _index_2))))
        (for _array_element_2 (.ParaList (Utilities|Struct|BreakST_EaseTweentoActionStruct (Utilities|Array|Get(acopy) (Variables|/Game/SpherePopupMenu/Blueprints/BP_EaseInstance.BP_EaseInstance_C|GetTweentoActionList _asbp_ease_instance) _index_2)))
          (Global|PlayTweento _array_element_2 1.0 (.Widget (Utilities|Struct|BreakST_EaseTweentoActionStruct (Utilities|Array|Get(acopy) (Variables|/Game/SpherePopupMenu/Blueprints/BP_EaseInstance.BP_EaseInstance_C|GetTweentoActionList _asbp_ease_instance) _index_2)))))
        (bind _asbp_menu_item (Utilities|Casting|CastToBP_MenuItem (.Widget (Utilities|Struct|BreakST_EaseTweentoActionStruct (Utilities|Array|Get(acopy) (Variables|/Game/SpherePopupMenu/Blueprints/BP_EaseInstance.BP_EaseInstance_C|GetTweentoActionList _asbp_ease_instance) _index_2)))))
        (Default|CallONTWEENTOEND _asbp_menu_item)
        (Utilities|Array|RemoveItem (Variables|/Game/SpherePopupMenu/Blueprints/BP_EaseInstance.BP_EaseInstance_C|GetTweentoActionList _asbp_ease_instance) (Utilities|Array|Get(acopy) (Variables|/Game/SpherePopupMenu/Blueprints/BP_EaseInstance.BP_EaseInstance_C|GetTweentoActionList _asbp_ease_instance) _index_2))))))

(fn GetCustomF
  (params (_s_sec :type Float%20%28single-precision%29) (_e_sec :type Float%20%28single-precision%29) (_c_ease :type E_EaseCustomEase%20Enum :default "NewEnumerator0"))
  (bind __c_f (Global|CalcCustomEase _c_ease (- (Utilities|Time|GetTimeSeconds) _s_sec) 0.0 1.0 (- _e_sec _s_sec)))
  (return __c_f))

(fn PlayWidgetTransform
  (params (_widget :type Widget%20Object%20Reference) (_dealy :type Float%20%28single-precision%29) (_translation_s :type Vector%202D%20Structure) (_translation_e :type Vector%202D%20Structure) (_scale_s :type Vector%202D%20Structure) (_scale_e :type Vector%202D%20Structure) (_shear_s :type Vector%202D%20Structure) (_shear_e :type Vector%202D%20Structure) (_c_ease :type E_EaseCustomEase%20Enum :default "NewEnumerator0"))
  (bind _para_list (LocalVariables|Getpara_list))
  (Utilities|Array|Add _para_list (Utilities|Struct|MakeST_EaseTweentoParaStruct false 0.0 0.0 false "(X=0.000000,Y=0.000000)" "(X=0.000000,Y=0.000000)" true _translation_s _translation_e _scale_s _scale_e _shear_s _shear_e false 0.0 0.0 false 1.0 1.0 false "(B=0,G=0,R=0,A=0)" "(B=0,G=0,R=0,A=0)" false (LocalVariables|Getbeziar_vec2ds)))
  (Custom|PlayWidgetMultipleProps _dealy _para_list _widget _c_ease))

(fn PlayWidgetScale
  (params (_widget :type Widget%20Object%20Reference) (_dealy :type Float%20%28single-precision%29) (_s :type Vector%202D%20Structure) (_e :type Vector%202D%20Structure) (_c_ease :type E_EaseCustomEase%20Enum :default "NewEnumerator0"))
  (bind _para_list (LocalVariables|Getpara_list))
  (Utilities|Array|Add _para_list (Utilities|Struct|MakeST_EaseTweentoParaStruct false 0.0 0.0 false "(X=0.000000,Y=0.000000)" "(X=0.000000,Y=0.000000)" true "(X=0.000000,Y=0.000000)" "(X=0.000000,Y=0.000000)" _s _e "(X=0.000000,Y=0.000000)" "(X=0.000000,Y=0.000000)" false 0.0 0.0 false 1.0 1.0 false "(B=0,G=0,R=0,A=0)" "(B=0,G=0,R=0,A=0)" false (LocalVariables|Getbeziar_vec2ds)))
  (Custom|PlayWidgetMultipleProps _dealy _para_list _widget _c_ease))

(fn PlayWidgetMultipleProps
  (params (_delay :type Float%20%28single-precision%29) (_para :type Array%20of%20ST%20Ease%20Tweento%20Para%20Struct%20Structures) (_widget :type Widget%20Object%20Reference) (_c_ease :type E_EaseCustomEase%20Enum :default "NewEnumerator0"))
  (bind _returnvalue (Utilities|Time|GetTimeSeconds))
  (bind _asbp_ease_instance (Utilities|Casting|CastToBP_EaseInstance (Game|GetGameInstance)))
  (Utilities|Array|Add (Variables|/Game/SpherePopupMenu/Blueprints/BP_EaseInstance.BP_EaseInstance_C|GetTweentoActionList _asbp_ease_instance) (Utilities|Struct|MakeST_EaseTweentoActionStruct _widget _returnvalue (+ _delay _returnvalue) _para _c_ease))
  (for _array_element _para
    (Global|PlayTweento _array_element 0.0 _widget)))

(fn PlayWidgetShear
  (params (_widget :type Widget%20Object%20Reference) (_dealy :type Float%20%28single-precision%29) (_s :type Vector%202D%20Structure) (_e :type Vector%202D%20Structure) (_c_ease :type E_EaseCustomEase%20Enum :default "NewEnumerator0"))
  (bind _para_list (LocalVariables|Getpara_list))
  (Utilities|Array|Add _para_list (Utilities|Struct|MakeST_EaseTweentoParaStruct false 0.0 0.0 false "(X=0.000000,Y=0.000000)" "(X=0.000000,Y=0.000000)" true "(X=0.000000,Y=0.000000)" "(X=0.000000,Y=0.000000)" "(X=1.000000,Y=1.000000)" "(X=1.000000,Y=1.000000)" _s _e false 0.0 0.0 false 1.0 1.0 false "(B=0,G=0,R=0,A=0)" "(B=0,G=0,R=0,A=0)" false (LocalVariables|Getbeziar_vec2ds)))
  (Custom|PlayWidgetMultipleProps _dealy _para_list _widget _c_ease))

(fn PlayWidgetVec2D
  (params (_widget :type Widget%20Object%20Reference) (_dealy :type Float%20%28single-precision%29) (_s :type Vector%202D%20Structure) (_e :type Vector%202D%20Structure) (_c_ease :type E_EaseCustomEase%20Enum :default "NewEnumerator0"))
  (bind _para_list (LocalVariables|Getpara_list))
  (Utilities|Array|Add _para_list (Utilities|Struct|MakeST_EaseTweentoParaStruct false 0.0 0.0 true _s _e false "(X=0.000000,Y=0.000000)" "(X=0.000000,Y=0.000000)" "(X=1.000000,Y=1.000000)" "(X=1.000000,Y=1.000000)" "(X=0.000000,Y=0.000000)" "(X=0.000000,Y=0.000000)" false 0.0 0.0 false 1.0 1.0 false "(B=0,G=0,R=0,A=0)" "(B=0,G=0,R=0,A=0)" false (LocalVariables|Getbeziar_vec2ds)))
  (Custom|PlayWidgetMultipleProps _dealy _para_list _widget _c_ease))

(fn PlayWidgetOpacity
  (params (_widget :type Widget%20Object%20Reference) (_dealy :type Float%20%28single-precision%29) (_s :type Float%20%28single-precision%29) (_e :type Float%20%28single-precision%29) (_c_ease :type E_EaseCustomEase%20Enum :default "NewEnumerator0"))
  (bind _para_list (LocalVariables|Getpara_list))
  (Utilities|Array|Add _para_list (Utilities|Struct|MakeST_EaseTweentoParaStruct false 0.0 0.0 false "(X=0.000000,Y=0.000000)" "(X=0.000000,Y=0.000000)" false "(X=0.000000,Y=0.000000)" "(X=0.000000,Y=0.000000)" "(X=1.000000,Y=1.000000)" "(X=1.000000,Y=1.000000)" "(X=0.000000,Y=0.000000)" "(X=0.000000,Y=0.000000)" false 0.0 0.0 true _s _e false "(B=0,G=0,R=0,A=0)" "(B=0,G=0,R=0,A=0)" false (LocalVariables|Getbeziar_vec2ds)))
  (Custom|PlayWidgetMultipleProps _dealy _para_list _widget _c_ease))

(fn PlayAngle
  (params (_para :type ST%20Ease%20Tweento%20Para%20Struct%20Structure) (_c_f :type Float%20%28single-precision%29) (_widget :type Widget%20Object%20Reference))
  (bind (_type_value _valuea _valueb _type_vector2d _vector2da _vector2db _type_transform _translationa _translationb _scalea _scaleb _sheara _shearb _type_angle _anglea _angleb) (Utilities|Struct|BreakST_EaseTweentoParaStruct _para))
  (if _type_angle
    (bind __res (Global|GetCustomEaseFloat _c_f _anglea _angleb))
    (Class|Widget|SetRenderTransformAngle _widget __res)))

(fn PlayWidgetAngle
  (params (_widget :type Widget%20Object%20Reference) (_dealy :type Float%20%28single-precision%29) (_s :type Float%20%28single-precision%29) (_e :type Float%20%28single-precision%29) (_c_ease :type E_EaseCustomEase%20Enum :default "NewEnumerator0"))
  (bind _para_list (LocalVariables|Getpara_list))
  (Utilities|Array|Add _para_list (Utilities|Struct|MakeST_EaseTweentoParaStruct false 0.0 0.0 false "(X=0.000000,Y=0.000000)" "(X=0.000000,Y=0.000000)" false "(X=0.000000,Y=0.000000)" "(X=0.000000,Y=0.000000)" "(X=1.000000,Y=1.000000)" "(X=1.000000,Y=1.000000)" "(X=0.000000,Y=0.000000)" "(X=0.000000,Y=0.000000)" true _s _e false 1.0 1.0 false "(B=0,G=0,R=0,A=0)" "(B=0,G=0,R=0,A=0)" false (LocalVariables|Getbeziar_vec2ds)))
  (Custom|PlayWidgetMultipleProps _dealy _para_list _widget _c_ease))

(fn PlayImageColorandOpacity
  (params (_image :type Image%20Object%20Reference) (_dealy :type Float%20%28single-precision%29) (_s :type Color%20Structure) (_e :type Color%20Structure) (_c_ease :type E_EaseCustomEase%20Enum :default "NewEnumerator0"))
  (bind _para_list (LocalVariables|Getpara_list))
  (Utilities|Array|Add _para_list (Utilities|Struct|MakeST_EaseTweentoParaStruct false 0.0 0.0 false "(X=0.000000,Y=0.000000)" "(X=0.000000,Y=0.000000)" false "(X=0.000000,Y=0.000000)" "(X=0.000000,Y=0.000000)" "(X=1.000000,Y=1.000000)" "(X=1.000000,Y=1.000000)" "(X=0.000000,Y=0.000000)" "(X=0.000000,Y=0.000000)" false 0.0 0.0 true 1.0 1.0 true _s _e false (LocalVariables|Getbeziar_vec2ds)))
  (Custom|PlayWidgetMultipleProps _dealy _para_list _image _c_ease))

(fn PlayColorandOpacity
  (params (_para :type ST%20Ease%20Tweento%20Para%20Struct%20Structure) (_c_f :type Float%20%28single-precision%29) (_widget :type Widget%20Object%20Reference))
  (bind (_type_value _valuea _valueb _type_vector2d _vector2da _vector2db _type_transform _translationa _translationb _scalea _scaleb _sheara _shearb _type_angle _anglea _angleb _type_opacity _opacitya _opacityb _type_color _colorveca _colorvecb) (Utilities|Struct|BreakST_EaseTweentoParaStruct _para))
  (if _type_color
    (bind __color (Global|GetCustomEaseColor _c_f _colorveca _colorvecb))
    (bind _asimage (Utilities|Casting|CastToImage _widget))
    (Appearance|SetColorandOpacity _asimage (Math|Conversions|ToLinearColor(Color) __color) :!class /Script/UMG.Image)))

(fn JieCheng
  (params (_int :type Integer))
  (for _index (range 1 _int)
    (LocalVariables|Setn (* _index (LocalVariables|Getn))))
  (return (LocalVariables|Getn)))

(fn CC
  (params (_n :type Integer) (_k :type Integer))
  (bind __res (Beziar|JieCheng _n))
  (LocalVariables|Setson __res)
  (bind __res_2 (Beziar|JieCheng _k))
  (bind __res_3 (Beziar|JieCheng (- _n _k)))
  (bind _output_get (LocalVariables|Setmom (* __res_2 __res_3)))
  (return (/ (Math|Conversions|ToFloat(Integer) (LocalVariables|Getson)) (Math|Conversions|ToFloat(Integer) _output_get))))

(fn BEZ
  (params (_n :type Integer) (_k :type Integer) (_t :type Float%20%28single-precision%29))
  (bind __res (Beziar|CC _n _k))
  (return (* __res (* (Math|Float|Power _t (Math|Conversions|ToFloat(Integer) _k)) (Math|Float|Power (- 1.0 _t) (Math|Conversions|ToFloat(Integer) (- _n _k)))))))

(fn PBEZ
  (params (_t :type Float%20%28single-precision%29) (pts :type Array%20of%20Vector%202D%20Structures))
  (bind _returnvalue (Utilities|Array|Length pts))
  (bind _returnvalue_2 (- _returnvalue 1))
  (for _index (range 0 _returnvalue_2)
    (bind __res (Beziar|BEZ _returnvalue_2 _index _t))
    (bind _output_get (LocalVariables|Set_b __res))
    (LocalVariables|Setx_p (+ (LocalVariables|Getx_p) (* _output_get (.X (Math|Vector2D|BreakVector2D (Utilities|Array|Get(acopy) pts _index))))))
    (LocalVariables|Sety_p (+ (LocalVariables|Gety_p) (* _output_get (.Y (Math|Vector2D|BreakVector2D (Utilities|Array|Get(acopy) pts _index)))))))
  (return (Math|Vector2D|MakeVector2D (LocalVariables|Getx_p) (LocalVariables|Gety_p))))

(fn PlayBeziar
  (params (_para :type ST%20Ease%20Tweento%20Para%20Struct%20Structure) (_c_f :type Float%20%28single-precision%29) (_widget :type Widget%20Object%20Reference))
  (bind (_type_value _valuea _valueb _type_vector2d _vector2da _vector2db _type_transform _translationa _translationb _scalea _scaleb _sheara _shearb _type_angle _anglea _angleb _type_opacity _opacitya _opacityb _type_color _colorveca _colorvecb _type_beziar _beziarvec2ds) (Utilities|Struct|BreakST_EaseTweentoParaStruct _para))
  (if _type_beziar
    (bind __res (Global|GetCustomEaseFloat _c_f 0.0 1.0))
    (bind __res_2 (Beziar|PBEZ __res _beziarvec2ds))
    (Class|CanvasPanelSlot|SetPosition (Class|WidgetLayoutLibrary|SlotasCanvasSlot _widget) __res_2)))

(fn PlayWidgetBeziar
  (params (_widget :type Widget%20Object%20Reference) (_dealy :type Float%20%28single-precision%29) (_beziar_vec2ds :type Array%20of%20Vector%202D%20Structures) (_c_ease :type E_EaseCustomEase%20Enum :default "NewEnumerator0"))
  (bind _para_list (LocalVariables|Getpara_list))
  (Utilities|Array|Add _para_list (Utilities|Struct|MakeST_EaseTweentoParaStruct false 0.0 0.0 true "(X=0.000000,Y=0.000000)" "(X=0.000000,Y=0.000000)" true "(X=0.000000,Y=0.000000)" "(X=0.000000,Y=0.000000)" "(X=1.000000,Y=1.000000)" "(X=1.000000,Y=1.000000)" "(X=0.000000,Y=0.000000)" "(X=0.000000,Y=0.000000)" false 0.0 0.0 false 1.0 1.0 false "(B=0,G=0,R=0,A=0)" "(B=0,G=0,R=0,A=0)" true _beziar_vec2ds))
  (Custom|PlayWidgetMultipleProps _dealy _para_list _widget _c_ease))

(fn CalcCustomEase
  (params (_c_ease :type E_EaseCustomEase%20Enum :default "NewEnumerator0") (_t :type Float%20%28single-precision%29) (_b :type Float%20%28single-precision%29) (_c :type Float%20%28single-precision%29) (_d :type Float%20%28single-precision%29))
  (bind _output_get (LocalVariables|Settmp_c_ease _c_ease))
  (LocalVariables|Settmp_t _t)
  (LocalVariables|Settmp_b _b)
  (LocalVariables|Settmp_c _c)
  (LocalVariables|Settmp_d _d)
  (switch Utilities|FlowControl|Switch|SwitchonE_EaseCustomEase _output_get
    (:NewEnumerator0
      (bind __res (CallFunction|StrongEasein (LocalVariables|Gettmp_t) (LocalVariables|Gettmp_b) (LocalVariables|Gettmp_c) (LocalVariables|Gettmp_d)))
      (return __res))
    (:NewEnumerator1
      (bind __res_2 (CallFunction|StrongEaseOut (LocalVariables|Gettmp_t) (LocalVariables|Gettmp_b) (LocalVariables|Gettmp_c) (LocalVariables|Gettmp_d)))
      (return __res_2))
    (:NewEnumerator2
      (bind __res_3 (CallFunction|StrongEaseinOut (LocalVariables|Gettmp_t) (LocalVariables|Gettmp_b) (LocalVariables|Gettmp_c) (LocalVariables|Gettmp_d)))
      (return __res_3))
    (:NewEnumerator3
      (bind __res_4 (CallFunction|SineEasein (LocalVariables|Gettmp_t) (LocalVariables|Gettmp_b) (LocalVariables|Gettmp_c) (LocalVariables|Gettmp_d)))
      (return __res_4))
    (:NewEnumerator4
      (bind __res_5 (CallFunction|SineEaseOut (LocalVariables|Gettmp_t) (LocalVariables|Gettmp_b) (LocalVariables|Gettmp_c) (LocalVariables|Gettmp_d)))
      (return __res_5))
    (:NewEnumerator5
      (bind __res_6 (CallFunction|SineEaseinOut (LocalVariables|Gettmp_t) (LocalVariables|Gettmp_b) (LocalVariables|Gettmp_c) (LocalVariables|Gettmp_d)))
      (return __res_6))
    (:NewEnumerator6
      (bind __res_7 (CallFunction|QuintEasein (LocalVariables|Gettmp_t) (LocalVariables|Gettmp_b) (LocalVariables|Gettmp_c) (LocalVariables|Gettmp_d)))
      (return __res_7))
    (:NewEnumerator7
      (bind __res_8 (CallFunction|QuintEaseOut (LocalVariables|Gettmp_t) (LocalVariables|Gettmp_b) (LocalVariables|Gettmp_c) (LocalVariables|Gettmp_d)))
      (return __res_8))
    (:NewEnumerator8
      (bind __res_9 (CallFunction|QuintEaseinOut (LocalVariables|Gettmp_t) (LocalVariables|Gettmp_b) (LocalVariables|Gettmp_c) (LocalVariables|Gettmp_d)))
      (return __res_9))
    (:NewEnumerator9
      (bind __res_10 (CallFunction|QuartEasein (LocalVariables|Gettmp_t) (LocalVariables|Gettmp_b) (LocalVariables|Gettmp_c) (LocalVariables|Gettmp_d)))
      (return __res_10))
    (:NewEnumerator10
      (bind __res_11 (CallFunction|QuartEaseOut (LocalVariables|Gettmp_t) (LocalVariables|Gettmp_b) (LocalVariables|Gettmp_c) (LocalVariables|Gettmp_d)))
      (return __res_11))
    (:NewEnumerator11
      (bind __res_12 (CallFunction|QuartEaseinOut (LocalVariables|Gettmp_t) (LocalVariables|Gettmp_b) (LocalVariables|Gettmp_c) (LocalVariables|Gettmp_d)))
      (return __res_12))
    (:NewEnumerator12
      (bind __res_13 (CallFunction|QuadEasein (LocalVariables|Gettmp_t) (LocalVariables|Gettmp_b) (LocalVariables|Gettmp_c) (LocalVariables|Gettmp_d)))
      (return __res_13))
    (:NewEnumerator13
      (bind __res_14 (CallFunction|QuadEaseOut (LocalVariables|Gettmp_t) (LocalVariables|Gettmp_b) (LocalVariables|Gettmp_c) (LocalVariables|Gettmp_d)))
      (return __res_14))
    (:NewEnumerator14
      (bind __res_15 (CallFunction|QuadEaseinOut (LocalVariables|Gettmp_t) (LocalVariables|Gettmp_b) (LocalVariables|Gettmp_c) (LocalVariables|Gettmp_d)))
      (return __res_15))
    (:NewEnumerator15
      (bind __res_16 (CallFunction|LinearEaseNone (LocalVariables|Gettmp_t) (LocalVariables|Gettmp_b) (LocalVariables|Gettmp_c) (LocalVariables|Gettmp_d)))
      (return __res_16))
    (:NewEnumerator16
      (bind __res_17 (CallFunction|LinearEasein (LocalVariables|Gettmp_t) (LocalVariables|Gettmp_b) (LocalVariables|Gettmp_c) (LocalVariables|Gettmp_d)))
      (return __res_17))
    (:NewEnumerator17
      (bind __res_18 (CallFunction|LinearEaseOut (LocalVariables|Gettmp_t) (LocalVariables|Gettmp_b) (LocalVariables|Gettmp_c) (LocalVariables|Gettmp_d)))
      (return __res_18))
    (:NewEnumerator18
      (bind __res_19 (CallFunction|LinearEaseinOut (LocalVariables|Gettmp_t) (LocalVariables|Gettmp_b) (LocalVariables|Gettmp_c) (LocalVariables|Gettmp_d)))
      (return __res_19))
    (:NewEnumerator19
      (bind __res_20 (CallFunction|ExpoEasein (LocalVariables|Gettmp_t) (LocalVariables|Gettmp_b) (LocalVariables|Gettmp_c) (LocalVariables|Gettmp_d)))
      (return __res_20))
    (:NewEnumerator20
      (bind __res_21 (CallFunction|ExpoEaseOut (LocalVariables|Gettmp_t) (LocalVariables|Gettmp_b) (LocalVariables|Gettmp_c) (LocalVariables|Gettmp_d)))
      (return __res_21))
    (:NewEnumerator21
      (bind __res_22 (CallFunction|ExpoEaseinOut (LocalVariables|Gettmp_t) (LocalVariables|Gettmp_b) (LocalVariables|Gettmp_c) (LocalVariables|Gettmp_d)))
      (return __res_22))
    (:NewEnumerator22
      (bind __res_23 (CallFunction|ElasticEasein (LocalVariables|Gettmp_t) (LocalVariables|Gettmp_b) (LocalVariables|Gettmp_c) (LocalVariables|Gettmp_d)))
      (return __res_23))
    (:NewEnumerator23
      (bind _res (CallFunction|ElasticEaseOut (LocalVariables|Gettmp_t) (LocalVariables|Gettmp_b) (LocalVariables|Gettmp_c) (LocalVariables|Gettmp_d)))
      (return _res))
    (:NewEnumerator24
      (bind __res_24 (CallFunction|ElasticEaseinOut (LocalVariables|Gettmp_t) (LocalVariables|Gettmp_b) (LocalVariables|Gettmp_c) (LocalVariables|Gettmp_d)))
      (return __res_24))
    (:NewEnumerator25
      (bind __res_25 (CallFunction|BackEasein (LocalVariables|Gettmp_t) (LocalVariables|Gettmp_b) (LocalVariables|Gettmp_c) (LocalVariables|Gettmp_d)))
      (return __res_25))
    (:NewEnumerator26
      (bind __res_26 (CallFunction|BackEaseOut (LocalVariables|Gettmp_t) (LocalVariables|Gettmp_b) (LocalVariables|Gettmp_c) (LocalVariables|Gettmp_d)))
      (return __res_26))
    (:NewEnumerator27
      (bind __res_27 (CallFunction|BackEaseinOut (LocalVariables|Gettmp_t) (LocalVariables|Gettmp_b) (LocalVariables|Gettmp_c) (LocalVariables|Gettmp_d)))
      (return __res_27))
    (:NewEnumerator28
      (bind __res_28 (CallFunction|BounceEasein (LocalVariables|Gettmp_t) (LocalVariables|Gettmp_b) (LocalVariables|Gettmp_c) (LocalVariables|Gettmp_d)))
      (return __res_28))
    (:NewEnumerator29
      (bind __res_29 (CallFunction|BounceEaseOut (LocalVariables|Gettmp_t) (LocalVariables|Gettmp_b) (LocalVariables|Gettmp_c) (LocalVariables|Gettmp_d)))
      (return __res_29))
    (:NewEnumerator30
      (bind __res_30 (CallFunction|BounceEaseinOut (LocalVariables|Gettmp_t) (LocalVariables|Gettmp_b) (LocalVariables|Gettmp_c) (LocalVariables|Gettmp_d)))
      (return __res_30))
    (:NewEnumerator31
      (bind __res_31 (CallFunction|CircEasein (LocalVariables|Gettmp_t) (LocalVariables|Gettmp_b) (LocalVariables|Gettmp_c) (LocalVariables|Gettmp_d)))
      (return __res_31))
    (:NewEnumerator32
      (bind __res_32 (CallFunction|CircEaseOut (LocalVariables|Gettmp_t) (LocalVariables|Gettmp_b) (LocalVariables|Gettmp_c) (LocalVariables|Gettmp_d)))
      (return __res_32))
    (:NewEnumerator33
      (bind __res_33 (CallFunction|CircEaseinOut (LocalVariables|Gettmp_t) (LocalVariables|Gettmp_b) (LocalVariables|Gettmp_c) (LocalVariables|Gettmp_d)))
      (return __res_33))
    (:NewEnumerator34
      (bind __res_34 (CallFunction|CubicEasein (LocalVariables|Gettmp_t) (LocalVariables|Gettmp_b) (LocalVariables|Gettmp_c) (LocalVariables|Gettmp_d)))
      (return __res_34))
    (:NewEnumerator35
      (bind __res_35 (CallFunction|CubicEaseOut (LocalVariables|Gettmp_t) (LocalVariables|Gettmp_b) (LocalVariables|Gettmp_c) (LocalVariables|Gettmp_d)))
      (return __res_35))
    (:NewEnumerator36
      (bind __res_36 (CallFunction|CubicEaseinOut (LocalVariables|Gettmp_t) (LocalVariables|Gettmp_b) (LocalVariables|Gettmp_c) (LocalVariables|Gettmp_d)))
      (return __res_36))))

(fn GetCustomEaseVec2D
  (params (_c_f :type Float%20%28single-precision%29) (_s :type Vector%202D%20Structure) (_e :type Vector%202D%20Structure))
  (return (+ (* (- _e _s) _c_f) _s)))

(fn GetCustomEaseFloat
  (params (_c_f :type Float%20%28single-precision%29) (_s :type Float%20%28single-precision%29) (_e :type Float%20%28single-precision%29))
  (return (+ (* _c_f (- _e _s)) _s)))

(fn GetCustomEaseVec3D
  (params (_c_f :type Float%20%28single-precision%29) (_s :type Vector) (_e :type Vector))
  (return (+ (* (- _e _s) _c_f) _s)))

(fn GetCustomEaseColor
  (params (_c_f :type Float%20%28single-precision%29) (_s :type Color%20Structure) (_e :type Color%20Structure))
  (bind (_b _g _r _a) (Math|Color|BreakColor _s))
  (bind (_b_2 _g_2 _r_2 _a_2) (Math|Color|BreakColor _e))
  (bind __res (Global|GetCustomEaseFloat _c_f (Math|Conversions|ToFloat(Byte) _b) (Math|Conversions|ToFloat(Byte) _b_2)))
  (bind __res_2 (Global|GetCustomEaseFloat _c_f (Math|Conversions|ToFloat(Byte) _g) (Math|Conversions|ToFloat(Byte) _g_2)))
  (bind __res_3 (Global|GetCustomEaseFloat _c_f (Math|Conversions|ToFloat(Byte) _r) (Math|Conversions|ToFloat(Byte) _r_2)))
  (bind __res_4 (Global|GetCustomEaseFloat _c_f (Math|Conversions|ToFloat(Byte) _a) (Math|Conversions|ToFloat(Byte) _a_2)))
  (return (Math|Conversions|ToColor(LinearColor) (Math|Color|MakeColor (/ __res_3 255.0) (/ __res_2 255.0) (/ __res 255.0) (/ __res_4 255.0)))))