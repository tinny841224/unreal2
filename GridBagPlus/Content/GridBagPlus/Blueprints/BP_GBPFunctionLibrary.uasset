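; Function library for GridBagPlus that runs a simple UI tween system on widget render scale or slot position.
; Tweens live in the game instance's TweenList, keyed by object name, with a flag allowing replacement of an existing one.
; TweenUpdata eases each entry by elapsed game time, clamping scale to 0–1, then removes finished entries.
; On reaching end time, a tween is flagged finished and calls GRIDTWEENEND with its BP_Grid widget.
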(fn TweenUpdata
  (Utilities|FlowControl|Sequence
    (:then_0
      (bind _asgbpgame_instance (CallFunction|GetBPGameInstance))
      (for _index (range 0 (- (Utilities|Array|Length (Variables|/Game/GridBagPlus/Blueprints/BP_GBPGameInstance.BP_GBPGameInstance_C|Gettween_list _asgbpgame_instance)) 1))
        (CallFunction|UpdataPerTween (Utilities|Array|Get(acopy) (Variables|/Game/GridBagPlus/Blueprints/BP_GBPGameInstance.BP_GBPGameInstance_C|Gettween_list _asgbpgame_instance) _index))))
    (:then_1
      (CallFunction|ClearOverTimeTween))))

(fn AddtoTweenList
  (params (_tween_data :type ST%20GBP%20Tween%20Data%20Structure) (abs :type Boolean))
  (bind _objectname (Utilities|Struct|BreakST_GBPTweenData _tween_data))
  (bind _exited (CallFunction|IsExistedTween _objectname))
  (if _exited
    (if abs
      (CallFunction|RemovefromTweenList _objectname)
      (bind _asgbpgame_instance (CallFunction|GetBPGameInstance :!label _label))
      (Utilities|Array|Add (Variables|/Game/GridBagPlus/Blueprints/BP_GBPGameInstance.BP_GBPGameInstance_C|Gettween_list _asgbpgame_instance) _tween_data))
    (else
      (goto _label))))

(fn IsExistedTween
  (params (tween_id :type String))
  (bind _asgbpgame_instance (CallFunction|GetBPGameInstance))
  (for _index (range 0 (- (Utilities|Array|Length (Variables|/Game/GridBagPlus/Blueprints/BP_GBPGameInstance.BP_GBPGameInstance_C|Gettween_list _asgbpgame_instance)) 1))
    (if (Utilities|Enum|Equal(Enum) tween_id (.ObjectName (Utilities|Struct|BreakST_GBPTweenData (Utilities|Array|Get(acopy) (Variables|/Game/GridBagPlus/Blueprints/BP_GBPGameInstance.BP_GBPGameInstance_C|Gettween_list _asgbpgame_instance) _index))))
      (return true)))
  (return false))

(fn GetBPGameInstance
  (bind _asbp_gbpgame_instance (Utilities|Casting|CastToBP_GBPGameInstance (Game|GetGameInstance)))
  (return _asbp_gbpgame_instance))

(fn RemovefromTweenList
  (params (tween_id :type String))
  (bind _asgbpgame_instance (CallFunction|GetBPGameInstance))
  (for _index (range 0 (- (Utilities|Array|Length (Variables|/Game/GridBagPlus/Blueprints/BP_GBPGameInstance.BP_GBPGameInstance_C|Gettween_list _asgbpgame_instance)) 1))
    (if (Utilities|Enum|Equal(Enum) tween_id (.ObjectName (Utilities|Struct|BreakST_GBPTweenData (Utilities|Array|Get(acopy) (Variables|/Game/GridBagPlus/Blueprints/BP_GBPGameInstance.BP_GBPGameInstance_C|Gettween_list _asgbpgame_instance) _index))))
      (Utilities|Array|RemoveItem (Variables|/Game/GridBagPlus/Blueprints/BP_GBPGameInstance.BP_GBPGameInstance_C|Gettween_list _asgbpgame_instance) (Utilities|Array|Get(acopy) (Variables|/Game/GridBagPlus/Blueprints/BP_GBPGameInstance.BP_GBPGameInstance_C|Gettween_list _asgbpgame_instance) _index)))))

(fn ClearOverTimeTween
  (bind _asgbpgame_instance (CallFunction|GetBPGameInstance))
  (for _array_element (Variables|/Game/GridBagPlus/Blueprints/BP_GBPGameInstance.BP_GBPGameInstance_C|Gettween_list _asgbpgame_instance)
    (if (.BOverTime (Utilities|Struct|BreakST_GBPTweenData _array_element))
      (Utilities|Array|RemoveItem (Variables|/Game/GridBagPlus/Blueprints/BP_GBPGameInstance.BP_GBPGameInstance_C|Gettween_list _asgbpgame_instance) _array_element))))

(fn UpdataPerTween
  (params (tween_data :type ST%20GBP%20Tween%20Data%20Structure%20%28by%20ref%29))
  (bind (_objectname _tweentype _bovertime _ssec _esec _lsec _ease _slot _widget) (Utilities|Struct|BreakST_GBPTweenData tween_data))
  (if (not _bovertime)
    (bind _f (CallFunction|GetTweenF _ssec _esec _lsec))
    (CallFunction|UpdataPerTweenData _f tween_data)
    (if (>= (Utilities|Time|GetTimeSeconds) _esec)
      (Utilities|Struct|SetmembersinST_GBPTweenData tween_data true)
      (bind _asgbpgame_instance (CallFunction|GetBPGameInstance))
      (bind _asbp_grid (Utilities|Casting|CastToBP_Grid _widget))
      (Default|CallGRIDTWEENEND _asgbpgame_instance _objectname _tweentype _asbp_grid))))

(fn GetTweenF
  (params (s :type Float%20%28single-precision%29) (e :type Float%20%28single-precision%29) (l :type Float%20%28single-precision%29))
  (bind _returnvalue (Utilities|Time|GetTimeSeconds))
  (if (>= _returnvalue e)
    (return 1.0)
    (else
      (return (/ (- _returnvalue s) l)))))

(fn UpdataPerTweenData
  (params (f :type Float%20%28single-precision%29) (tween_data :type ST%20GBP%20Tween%20Data%20Structure%20%28by%20ref%29))
  (bind (_objectname _tweentype _bovertime _ssec _esec _lsec _ease _slot _widget _bwidgetscale _swidgetscale _ewidgetscale _bslotpos) (Utilities|Struct|BreakST_GBPTweenData tween_data))
  (if _bwidgetscale
    (CallFunction|TweenWidgetScale f tween_data)
    (elif _bslotpos
      (CallFunction|TweenSlotPos f tween_data))))

(fn TweenWidgetScale
  (params (f :type Float%20%28single-precision%29) (tween_data :type ST%20GBP%20Tween%20Data%20Structure%20%28by%20ref%29))
  (bind (_objectname _tweentype _ease _slot _widget _bwidgetscale _swidgetscale _ewidgetscale) (Utilities|Struct|BreakST_GBPTweenData tween_data))
  (bind (_x _y) (Math|Vector2D|BreakVector2D _swidgetscale))
  (bind (_x_2 _y_2) (Math|Vector2D|BreakVector2D _ewidgetscale))
  (bind _out (CallFunction|Format01 (Math|Interpolation|Ease _ease f _x _x_2 2.0)))
  (bind _out_2 (CallFunction|Format01 (Math|Interpolation|Ease _ease f _y _y_2 2.0)))
  (Widget|Transform|SetRenderScale _widget (Math|Vector2D|MakeVector2D _out _out_2)))

(fn TweenSlotPos
  (params (f :type Float%20%28single-precision%29) (tween_data :type ST%20GBP%20Tween%20Data%20Structure%20%28by%20ref%29))
  (bind (_objectname _tweentype _ease _slot _widget _bwidgetscale _swidgetscale _ewidgetscale _bslotpos _sslotpos _eslotpos) (Utilities|Struct|BreakST_GBPTweenData tween_data))
  (bind (_x _y) (Math|Vector2D|BreakVector2D _sslotpos))
  (bind (_x_2 _y_2) (Math|Vector2D|BreakVector2D _eslotpos))
  (Class|CanvasPanelSlot|SetPosition _slot (Math|Vector2D|MakeVector2D (Math|Interpolation|Ease _ease f _x _x_2 2.0) (Math|Interpolation|Ease _ease f _y _y_2 2.0))))

(fn Format01
  (params (in :type Float%20%28single-precision%29))
  (if (<= in 0.0)
    (return 0.0)
    (elif (>= in 1.0)
      (return 1.0)
      (else
        (return in)))))